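; Shower bolt-action puzzle module whose core tube rotates to find a target angle, then pops out and shoves back in.
; BeginPlay randomizes stage spots and starting rotation, but only the first spot becomes the target.
; While hovered, left or other mouse clicks drive opposite timeline rotations, gated by cursor X.
; Landing on the target advances the state through pop-out, shove-in and completion, which only prints debug text.
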(event `self.ReceiveBeginPlay`
  (bind _returnvalue (`KismetMathLibrary.RandomInteger` 3))
  (bind _returnvalue_2 (`KismetMathLibrary.RandomInteger` 2))
  (bind _returnvalue_3 (`KismetMathLibrary.Conv_IntToDouble` (`|GetArrayItem` (`self.ValidSpots`) (`KismetMathLibrary.RandomInteger` 1))))
  (`KismetSystemLibrary.Delay` 0.2)
  (bind _output_get (set `self.Stage1CorrectSpot` (`|GetArrayItem` (`self.ValidSpots`) _returnvalue)))
  (set `self.TargetRotation` (`KismetMathLibrary.Conv_IntToDouble` _output_get))
  (`KismetArrayLibrary.Array_Remove` (`self.ValidSpots`) _returnvalue)
  (set `self.Stage2CorrectSpot` (`|GetArrayItem` (`self.ValidSpots`) _returnvalue_2))
  (`KismetArrayLibrary.Array_Remove` (`self.ValidSpots`) _returnvalue_2)
  (set `self.Stage3CorrectSpot` (`|GetArrayItem` (`self.ValidSpots`) (`KismetMathLibrary.RandomInteger` 1)))
  (`SceneComponent.K2_SetRelativeRotation` (`self.CoreTube`) (`KismetMathLibrary.MakeRotator` 0.0 _returnvalue_3) false false)
  (set `self.LastRotation` _returnvalue_3))

(event `self.ReceiveActorBeginCursorOver`
  (set `self.IsActive` true))

(event `self.ReceiveActorEndCursorOver`
  (set `self.IsActive` false))

(event `Key|LeftMouseButton`
  (params (Key :type "Key Structure"))
  (:`Pressed`
    (if (`self.IsActive`) :!label _label
      (set `self.BeingUsed` true)
      (bind _returnvalue (`WidgetLayoutLibrary.GetMousePositionOnPlatform`))
      (if (and (>= (- (`KismetMathLibrary.BreakVector2D` _returnvalue) (`KismetMathLibrary.BreakVector2D` (0.0 0.0))) 30.0) (`self.BeingUsed`))
        (`self.RotateModuleLeft`))
      (else
        (`KismetSystemLibrary.PrintString` "How did this happen?")))))

(event `PopOut`
  ;[1 1 1] Pop Out Logic
  (bind (_direction _newtrack_0) (`Timeline|PopOutTimeline` :!via `PlayFromStart`)
    (:`Update`
      (`SceneComponent.K2_SetRelativeLocation` (`self.CoreTube`) (`KismetMathLibrary.MakeVector` 0.0 _newtrack_0) false false))))

(event `self.ReceiveActorOnClicked`
  (params (ButtonPressed :type "Key Structure"))
  (bind _output_get (set `self.WhyIsThisNecessary` ButtonPressed))
  (if (== _output_get "LeftMouseButton")
    (goto _label)
    (elif (`self.IsActive`)
      (set `self.BeingUsed` true)
      (bind _returnvalue (`WidgetLayoutLibrary.GetMousePositionOnPlatform`))
      (if (and (>= (- (`KismetMathLibrary.BreakVector2D` _returnvalue) (`KismetMathLibrary.BreakVector2D` (0.0 0.0))) 30.0) (`self.BeingUsed`))
        (`self.RotateModuleRight`))
      (else
        (`KismetSystemLibrary.PrintString` "How did this happen?")))))

(event `ShoveIn`
  ;[1 1 1] Shove In Logic
  (bind (_direction _newtrack_0) (`Timeline|ShoveInTimeline` :!via `PlayFromStart`)
    (:`Update`
      (`SceneComponent.K2_SetRelativeLocation` (`self.CoreTube`) (`KismetMathLibrary.MakeVector` 0.0 _newtrack_0) false false))))

(event `RotateModuleLeft`
  (bind _coretube (`self.CoreTube`))
  ;[1 1 1] If ending pos = correct spot, continue to next stage.
  (bind (_direction _rotate) (`Timeline|Timeline_0` :`NewTime` 1.0 :!via `ReverseFromEnd`)
    (:`Update`
      (bind _returnvalue (`KismetMathLibrary.MakeRotator` 0.0 (+ _rotate (`self.LastRotation`))))
      (`SceneComponent.K2_SetRelativeRotation` _coretube _returnvalue false false))
    (:`Finished`
      (if (< (`self.LastRotation`) 0.0)
        (`SceneComponent.K2_SetRelativeRotation` :`self` _coretube)
        (set `self.LastRotation` 270.0)
        (else
          (set `self.LastRotation` (.pitch _returnvalue))))
      (if (== (`self.LastRotation`) (`self.TargetRotation`))
        (set `self.CurrentState` (+ (`self.CurrentState`) 1))
        (`KismetSystemLibrary.PrintString` "next stage")
        (if (== (`self.CurrentState`) 1)
          (`self.PopOut`)
          (elif (== (`self.CurrentState`) 2)
            (`self.ShoveIn`)
            (else
              (`KismetSystemLibrary.PrintString` "Module Complete"))))))))

(event `RotateModuleRight`
  (bind _coretube (`self.CoreTube`))
  ;[1 1 1] If ending pos = correct spot, continue to next stage.
  (bind (_direction _rotate) (`Timeline|Timeline_1` :`NewTime` 1.0 :!via `PlayFromStart`)
    (:`Update`
      (bind _returnvalue (`KismetMathLibrary.MakeRotator` 0.0 (+ _rotate (`self.LastRotation`))))
      (`SceneComponent.K2_SetRelativeRotation` _coretube _returnvalue false false))
    (:`Finished`
      (if (> (`self.LastRotation`) 359.0)
        (`SceneComponent.K2_SetRelativeRotation` :`self` _coretube)
        (set `self.LastRotation` 0.0)
        (else
          (set `self.LastRotation` (.pitch _returnvalue))))
      (if (== (`self.LastRotation`) (`self.TargetRotation`))
        (set `self.CurrentState` (+ (`self.CurrentState`) 1))
        (`KismetSystemLibrary.PrintString` "next stage")
        (if (== (`self.CurrentState`) 1)
          (`self.PopOut`)
          (elif (== (`self.CurrentState`) 2)
            (`self.ShoveIn`)
            (else
              (`self.BoltActionComplete`))))))))

(event `BoltActionComplete`
  (`KismetSystemLibrary.PrintString` "Confetti"))

(fn `UserConstructionScript`)