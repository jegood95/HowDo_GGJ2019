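; Scrolly is an actor in the Microwave folder that maps its position to a wave type, apparently as a selector.
; Each Tick it prints WaveState, then compares its Y location against evenly spaced stops to set Radio, Micro, Light, XRay or Gamma.
; When Y is outside every stop's tolerance, it moves the actor back to a hardcoded position at the Radio stop.
; The movement between stops is not handled here.
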(event `self.ReceiveTick`
  (params (DeltaSeconds :type "Float (single-precision)"))
  (bind _y (.y (`self.K2_GetActorLocation`)))
  (`KismetSystemLibrary.PrintString` (`self.WaveState`))
  (if (`KismetMathLibrary.NearlyEqual_FloatFloat` _y 20.0 1.0)
    (set `self.WaveState` "Radio")
    (elif (`KismetMathLibrary.NearlyEqual_FloatFloat` _y 23.0 1.0)
      (set `self.WaveState` "Micro")
      (elif (`KismetMathLibrary.NearlyEqual_FloatFloat` _y 26.0 1.0)
        (set `self.WaveState` "Light")
        (elif (`KismetMathLibrary.NearlyEqual_FloatFloat` _y 29.0 1.0)
          (set `self.WaveState` "XRay")
          (elif (`KismetMathLibrary.NearlyEqual_FloatFloat` _y 32.0 1.0)
            (set `self.WaveState` "Gamma")
            (else
              (`self.K2_SetActorLocation` (-194.043289 20.0 247.0)))))))))

(fn `UserConstructionScript`)